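; Instanced foliage mesh that the player chops to harvest items, such as wood from trees, with health tracked per instance.
; BeginPlay caches the player's inventory after a short delay and fills a health array indexed by instance.
; Chop damages the hit instance and adds a random amount of its data table item on every hit.
; It plays a tree-fall sound and removes the instance when updated health minus Damage again reaches zero.
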(event EventBeginPlay
  (Utilities|FlowControl|Delay 0.2)
  (bind _asbp_first_person_character (Utilities|Casting|CastToBP_FirstPersonCharacter (Game|GetPlayerCharacter 0)))
  (Variables|Default|SetInventory%20Component (Variables|/Script/SurvivalGame.SurvivalCharacter|GetInventoryComponent _asbp_first_person_character))
  (for _index (range 0 (Components|InstancedStaticMesh|GetInstanceCount))
    (Utilities|Array|SetArrayElem (Variables|Default|GetFoliageHealth) _index (Utilities|Struct|MakeS_FoliageHealth 1e+02) true)))

(event EventChop
  (params (Damage :type Float%20%28single-precision%29) (HitResult :type Hit%20Result%20Structure))
  (bind _hititem (Collision|BreakHitResult HitResult))
  (bind _foliagehealth (Variables|Default|GetFoliageHealth))
  (bind _datatablerow (Variables|Default|GetDataTableRow))
  (bind _output (Utilities|Array|Get(acopy) _foliagehealth _hititem))
  (bind _returnvalue (- (.health _output) Damage))
  (Utilities|Array|SetArrayElem _foliagehealth _hititem (Utilities|Struct|MakeS_FoliageHealth _returnvalue))
  (bind _returnvalue_2 (Utilities|GetDataTableRow (.datatable _datatablerow) (.rowname _datatablerow))
    (:then
      (Class|InventoryComponent|AddItem (Variables|Default|GetInventory%20Component) (Utilities|Struct|MakeItemData (.Name (Utilities|Struct|BreakItemData _returnvalue_2)) (Math|Random|RandomIntegerinRange 2 5) (.StaticMesh (Utilities|Struct|BreakItemData _returnvalue_2)) (.Icon (Utilities|Struct|BreakItemData _returnvalue_2)) (.bCanCraft (Utilities|Struct|BreakItemData _returnvalue_2))))
      (if (<= _returnvalue 0.0)
        (Audio|PlaySoundatLocation "/Game/Audio/Sounds/MS_TreeFall.MS_TreeFall" (.location (.OutInstanceTransform (Components|InstancedStaticMesh|GetInstanceTransform _hititem false))) "0, 0, 0" 1.0 1.0 0.0 0 0 0 0)
        (Class|InstancedStaticMeshComponent|RemoveInstance _hititem)))))