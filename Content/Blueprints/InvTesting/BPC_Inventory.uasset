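; Inventory component that stores item structs in an array and toggles the inventory screen.
; The inventory input creates WBP_Inventory or closes it, switching cursor visibility and input mode with a window sound.
; AddItem stacks items by name or appends new entries.
; RemoveItem subtracts one or the given amount, deleting depleted entries and returning true only on that deletion path.
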(event Custom|CloseInventory
  (bind _returnvalue (Game|GetPlayerController 0))
  (Widget|RemovefromParent (Variables|Default|GetInventoryWidget))
  (Variables|Default|SetInventoryWidget 0)
  (Variables|/Script/Engine.PlayerController|SetbShowMouseCursor _returnvalue false)
  (Input|SetInputModeGameOnly _returnvalue false)
  (Audio|PlaySound2D "/Engine/VREditor/Sounds/UI/Dockable_Window_Close.Dockable_Window_Close" 1.0 1.0 0.0 0 0))

(event Input|EnhancedActionEvents|EnhancedInputActionIA_Inventory
  (params (ActionValue :type Boolean) (ElapsedSeconds :type Float%20%28double-precision%29) (TriggeredSeconds :type Float%20%28double-precision%29) (InputAction :type Input%20Action%20Object%20Reference :default "/Game/Input/Actions/IA_Inventory.IA_Inventory"))
  (bind _returnvalue (Game|GetPlayerController 0))
  (bind _returnvalue_2 (Game|GetPlayerController 0))
  (:Started
    (Variables|Default|GetInventoryWidget
      (:then
        (Widget|RemovefromParent (Variables|Default|GetInventoryWidget))
        (Variables|Default|SetInventoryWidget 0)
        (Variables|/Script/Engine.PlayerController|SetbShowMouseCursor _returnvalue false)
        (Input|SetInputModeGameOnly _returnvalue false)
        (Audio|PlaySound2D "/Engine/VREditor/Sounds/UI/Dockable_Window_Close.Dockable_Window_Close" 1.0 1.0 0.0 0 0))
      (:else
        (bind _returnvalue_3 (UserInterface|CreateWidget "/Game/Blueprints/UI/Inventory/WBP_Inventory.WBP_Inventory_C"))
        (bind _output_get (Variables|Default|SetInventoryWidget _returnvalue_3))
        (UserInterface|Viewport|AddtoViewport _output_get 0)
        (Variables|/Script/Engine.PlayerController|SetbShowMouseCursor _returnvalue_2 true)
        (Input|SetInputModeGameandUI _returnvalue_2 0 "DoNotLock" true false)
        (Audio|PlaySound2D "/Engine/VREditor/Sounds/UI/Dockable_Window_Open.Dockable_Window_Open" 1.0 1.0 0.0 0 0)))))

(fn AddItem
  (params (NewItem :type S%20Item%20Structure))
  (bind (_name _amount _staticmesh _icon _cancraft) (Utilities|Struct|BreakS_Item NewItem))
  (bind (_array_element _array_index) (Utilities|Array|ForEachLoopwithBreak (Variables|Default|Getitems) :!label _label)
    (:LoopBody
      (if (Utilities|Enum|Equal(Enum) (.Name (Utilities|Struct|BreakS_Item _array_element)) _name)
        ;[0.15 0.15 0.15 0.5] Stack Item
        (Utilities|Array|SetArrayElem (Variables|Default|Getitems) _array_index (Utilities|Struct|MakeS_Item _name (+ (.Amount (Utilities|Struct|BreakS_Item _array_element)) _amount) _staticmesh _icon _cancraft))
        (LocalVariables|SetExistingItem true)
        (goto _label Break)))
    (:Completed
      ;[0.15 0.15 0.15 0.5] New Item
      (if (not (LocalVariables|GetExistingItem))
        (Utilities|Array|Add (Variables|Default|Getitems) NewItem)))))

(fn RemoveItem
  (params (Item :type S%20Item%20Structure) (DecreaseOneOnly :type Boolean))
  (bind (_name _amount) (Utilities|Struct|BreakS_Item Item))
  (bind (_name_2 _amount_2 _staticmesh _icon _cancraft) (Utilities|Struct|BreakS_Item Item))
  (bind (_array_element _array_index) (Utilities|Array|ForEachLoopwithBreak (Variables|Default|Getitems) :!label _label)
    (:LoopBody
      (LocalVariables|SetArrayIndex _array_index)
      (if (Utilities|Enum|Equal(Enum) (.Name (Utilities|Struct|BreakS_Item _array_element)) _name)
        (if (< (.Amount (Utilities|Struct|BreakS_Item _array_element)) 2)
          _
          (elif (> (- (.Amount (Utilities|Struct|BreakS_Item _array_element)) (Math|Integer|SelectInt 1 _amount DecreaseOneOnly)) 0)
            (Utilities|Array|SetArrayElem (Variables|Default|Getitems) (LocalVariables|GetArrayIndex) (Utilities|Struct|MakeS_Item _name_2 (- (.Amount (Utilities|Struct|BreakS_Item _array_element)) (Math|Integer|SelectInt 1 _amount DecreaseOneOnly)) _staticmesh _icon _cancraft))
            (goto _label Break)
            (else
              _)))
        (Utilities|Array|RemoveIndex (Variables|Default|Getitems) (LocalVariables|GetArrayIndex))
        (Utilities|FlowControl|Sequence
          (:then_0
            (goto _label Break))
          (:then_1
            (return true)))))))